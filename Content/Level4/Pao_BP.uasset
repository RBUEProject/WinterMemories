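; Level 4 cannon (Pao) that launches Botton_Bp actors at random intervals while the level's Starter actor has Start set.
; Tick polls the first Starter and uses a random Delay as a repeating timer, spawning at the Scene component's transform with a teleport sound and particle activation.
; When Start is off, it stops the last spawned sound and hides the particles, provided that sound is still valid.
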(event `self.ReceiveBeginPlay`
  (bind (_returnvalue_roll _returnvalue_pitch _returnvalue_yaw) (`KismetMathLibrary.BreakRotator` (`self.K2_GetActorRotation`)))
  (`self.K2_SetActorRotation` (`KismetMathLibrary.MakeRotator` _returnvalue_roll _returnvalue_pitch _returnvalue_yaw)))

(event `self.ReceiveTick`
  (params (DeltaSeconds :type "Float (single-precision)"))
  (bind _particlesystem (`self.ParticleSystem`))
  (bind _outactors (`GameplayStatics.GetAllActorsOfClass` "/Game/Starter.Starter_C"))
  (if (`/Game/Starter.Start?` (`|GetArrayItem` _outactors))
    (`KismetSystemLibrary.Delay` (`KismetMathLibrary.RandomFloatInRange` 1.0 5.0))
    (`|SpawnActorFromClass` "/Game/Level4/botton_Bp.botton_Bp_C" (`SceneComponent.K2_GetComponentToWorld` (`self.Scene`)) "Undefined" "OverrideRootScale" null null)
    (bind _returnvalue (`GameplayStatics.SpawnSoundAtLocation` "/Engine/VREditor/Sounds/UI/Teleport_Committed.Teleport_Committed" (`self.K2_GetActorLocation`) (struct) 1.0 1.0 0.0 null null))
    (`ActorComponent.SetActive` _particlesystem true false)
    (else
      (`/Engine/EditorBlueprintResources/StandardMacros.IsValid` _returnvalue
        (:`Is Valid`
          (`AudioComponent.Stop` _returnvalue)
          (`/Engine/EditorBlueprintResources/StandardMacros.IsValid` _particlesystem
            (:`Is Valid`
              (`SceneComponent.SetHiddenInGame` _particlesystem true false))))))))

(fn `UserConstructionScript`)