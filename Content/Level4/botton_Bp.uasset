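; Short-lived rolling or flying projectile actor for Level4 that carries a snowball effect.
; On BeginPlay it sets the Sphere's physics velocity along its right vector, attaches the SnowBall FX system and limits its own lifespan to a few seconds.
; Each Tick it looks up the first Starter actor and shows or hides both sphere and effect according to that actor's Start flag.
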(event `self.ReceiveBeginPlay`
  (bind _sphere (`self.Sphere`))
  (`PrimitiveComponent.SetPhysicsLinearVelocity` _sphere (* (`KismetMathLibrary.GetRightVector` (`SceneComponent.K2_GetComponentRotation` _sphere)) 1300.0) false "None")
  (`self.SetLifeSpan` 5.0)
  (bind _returnvalue (`NiagaraFunctionLibrary.SpawnSystemAttached` "/Game/fx/FX_Snow/Particles/SnowBall_FX_System.SnowBall_FX_System" (`self.Sphere`) "None" (0.0 0.0 0.0) (struct) "KeepRelativeOffset")))

(event `self.ReceiveTick`
  (params (DeltaSeconds :type "Float (single-precision)"))
  (bind _outactors (`GameplayStatics.GetAllActorsOfClass` "/Game/Starter.Starter_C"))
  (if (`/Game/Starter.Start?` (`|GetArrayItem` _outactors))
    (`SceneComponent.SetHiddenInGame` (`self.Sphere`) false false)
    (`SceneComponent.SetHiddenInGame` (stale `self.ReceiveBeginPlay` _returnvalue) false false)
    (else
      (`SceneComponent.SetHiddenInGame` (`self.Sphere`) true false)
      (`SceneComponent.SetHiddenInGame` (stale `self.ReceiveBeginPlay` _returnvalue) true false))))

(fn `UserConstructionScript`)